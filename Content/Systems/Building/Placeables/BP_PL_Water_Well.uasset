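; Placeable water well that players drink from, holding a limited number of charges that regenerate over time.
; A one-second looping timer refills charges at a per-minute rate once placed, skipping brush previews.
; Interacting feeds the pawn's hunger system, spends a charge and logs a server-side journey event, while RefillFromWaterwell lets callers spend one too.
; The water mesh slides between two spline points by charge ratio and hides below one charge.
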(event Custom|TickCharges
  (Utilities|And+Branch (Variables|Default|GetHasBeenPlacedInWorld) (< (Variables|Default|GetCurDrinkCharges) (Variables|Default|GetMaxDrinkCharges)) ; Make sure wells do not fill themselves when they are in brush mode
    (:True
      (Variables|Default|SetCurDrinkCharges (+ (Variables|Default|GetCurDrinkCharges) (/ (Variables|Default|GetRefillRate) 6e+01)))
      (Variables|Default|SetCurDrinkCharges (Math|Float|Clamp(Float) (Variables|Default|GetCurDrinkCharges) 0.0 (Variables|Default|GetMaxDrinkCharges)))
      (if (not (Networking|IsDedicatedServer))
        (CallFunction|UpdateWaterPositionandVisibility)))))

(event Custom|ForceUpdateWellStatus
  (CallFunction|UpdateWaterPositionandVisibility))

(event EventInteractableActivate
  (params (Component :type Primitive%20Component%20Object%20Reference) (Instigator :type Player%20Controller%20Object%20Reference) (HitIndex :type Integer))
  (bind _returnvalue (Pawn|GetControlledPawn Instigator))
  (bind _returnvalue_2 (Actor|GetComponentsByClass _returnvalue "/Game/Systems/Hunger/BP_HungerSystem.BP_HungerSystem_C"))
  (if (> (Utilities|Array|Length _returnvalue_2) 0)
    (if (CallFunction|GetCanDrink)
      (Default|ServerDrink (Utilities|Array|Get(acopy) _returnvalue_2) (Variables|Default|GetOnInteractDrinkValue))
      (CallFunction|DecrementDrinkCharges)
      (CallFunction|ForceUpdateWellStatus)
      (CallFunction|UpdateJourneyEvent Instigator))))

(event EventBeginPlay
  (|CallParentFunction)
  (CallFunction|UpdateWaterPositionandVisibility)
  (if (not (Variables|Default|GetIsABrush))
    (Utilities|Time|SetTimerbyEvent (delegate Custom|TickCharges) 1.0 true)))

(fn ConstructionScript
  (|CallParentFunction))

(fn UpdateWaterPositionandVisibility
  (if (< (Variables|Default|GetCurDrinkCharges) 1.0)
    (Rendering|SetVisibility (Variables|Default|GetWaterMesh) false false)
    (else
      (Rendering|SetVisibility (Variables|Default|GetWaterMesh) true false)))
  (Transformation|SetWorldLocation (Variables|Default|GetWaterMesh) (Math|Vector|Lerp(Vector) (Spline|GetLocationatSplinePoint (Variables|Default|GetWaterSpline) 0 "World") (Spline|GetLocationatSplinePoint (Variables|Default|GetWaterSpline) 1 "World") (/ (Variables|Default|GetCurDrinkCharges) (Variables|Default|GetMaxDrinkCharges))) false false))

(fn DecrementDrinkCharges
  (Math|Float|DecrementFloat (Variables|Default|GetCurDrinkCharges)
    (:%20%20
      (CallFunction|UpdateWaterPositionandVisibility)
      (return))))

(fn GetCanDrink
  (return (> (Variables|Default|GetCurDrinkCharges) 1.0)))

(fn UpdateJourneyEvent
  (params (Instigator :type Player%20Controller%20Object%20Reference))
  (if (Networking|IsServer)
    (bind _asbase_player_char_interface (Utilities|Casting|CastToBasePlayerCharInterface (Pawn|GetControlledPawn Instigator)))
    (Default|AddJourneyEventInterfaceCall _asbase_player_char_interface "DrinkFromWell")))

(fn RefillfromWaterwell
  (if (CallFunction|GetCanDrink)
    (CallFunction|DecrementDrinkCharges)
    (return true)
    (else
      (return false))))