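; Perk component for Conan characters that grants attribute perks and supplies their gameplay modifiers.
; It evaluates each data table row against an int or float stat range, updating owned perks and firing a server-side journey event when one qualifies.
; On the server, database-loaded characters wait for persistence data before applying perks.
; Getters expose combat, stamina and other modifiers, some perk-gated, with damage bonuses summed from attack type, status effects, encumbrance and headshots.
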(event Custom|SlotDataLoaded
  (Class|PerkSystemComponent|ApplyAllPerks)
  (Default|CallOnPerksLoaded))

(event EventBeginPlay
  (|CallParentFunction)
  (if (Networking|IsServer)
    (bind _asconan_character (Utilities|Casting|CastToConanCharacter (Components|GetOwner)))
    (if (Variables|/Script/UE4Dreamworld.PersistenceComponent|Getm_bWasLoadedFromDB (Actor|GetComponentbyClass _asconan_character "/Script/UE4Dreamworld.ActorPersistenceComponent"))
      (EventDispatchers|AssignOnSignalDataLoaded (Actor|GetComponentbyClass _asconan_character "/Script/UE4Dreamworld.ActorPersistenceComponent") (delegate Custom|SlotDataLoaded))
      (else
        (Class|PerkSystemComponent|ApplyAllPerks :!label _label)
        (Default|CallOnPerksLoaded)))
    (else
      (goto _label))))

(event EventApplyAllPerks
  (|CallParentFunction)
  (Class|PerkSystemComponent|ClearAllOwnedPerks)
  (bind _outrownames (DataTable|GetDataTableRowNames "/Game/Systems/Perks/PerkDataTable.PerkDataTable"))
  (for _array_element _outrownames
    (CallFunction|CheckandApplyPerk _array_element)))

(event EventUpdatePerkStatus
  (params (Perks :type Array%20of%20Names))
  (for _array_element Perks
    (CallFunction|CheckandApplyPerk _array_element)))

(fn CheckandApplyPerk
  (params (Perk :type Name))
  (bind _output_get (LocalVariables|SetinPerk Perk))
  (Class|PerkSystemComponent|RemoveOwnedPerk _output_get)
  (bind _returnvalue (Utilities|GetDataTableRow "/Game/Systems/Perks/PerkDataTable.PerkDataTable" (LocalVariables|GetinPerk))
    (:then
      (bind _asconan_character (Utilities|Casting|CastToConanCharacter (Components|GetOwner))
        (:then
          (if (.UseIntStat (Utilities|Struct|BreakST_PerkEntry _returnvalue))
            (Class|PerkSystemComponent|RegisterSeenIntPerkStat (.TargetIntStat (Utilities|Struct|BreakST_PerkEntry _returnvalue)) (LocalVariables|GetinPerk))
            (if (Math|Float|InRange(Float) (Math|Conversions|ToFloat(Integer) (Class|ConanCharacter|GetIntStat _asconan_character (.TargetIntStat (Utilities|Struct|BreakST_PerkEntry _returnvalue)) "Full")) (.Min (Utilities|Struct|BreakSpawnTableRange (.Limit (Utilities|Struct|BreakST_PerkEntry _returnvalue)))) (.Max (Utilities|Struct|BreakSpawnTableRange (.Limit (Utilities|Struct|BreakST_PerkEntry _returnvalue)))))
              (Class|PerkSystemComponent|AddOwnedPerk (LocalVariables|GetinPerk))
              (else
                (return false)))
            (else
              (Class|PerkSystemComponent|RegisterSeenFloatPerkStat (.TargetFloatStat (Utilities|Struct|BreakST_PerkEntry _returnvalue)) (LocalVariables|GetinPerk))
              (if (Math|Float|InRange(Float) (Class|ConanCharacter|GetFloatStat _asconan_character (.TargetFloatStat (Utilities|Struct|BreakST_PerkEntry _returnvalue)) "Full") (.Min (Utilities|Struct|BreakSpawnTableRange (.Limit (Utilities|Struct|BreakST_PerkEntry _returnvalue)))) (.Max (Utilities|Struct|BreakSpawnTableRange (.Limit (Utilities|Struct|BreakST_PerkEntry _returnvalue)))))
                (Class|PerkSystemComponent|AddOwnedPerk (LocalVariables|GetinPerk))
                (else
                  (return false)))))
          (CallFunction|GiveJourneyEvent)
          (return true))
        (:CastFailed
          (return false))))
    (:RowNotFound
      (return false))))

(fn GiveJourneyEvent
  (if (Networking|IsServer)
    (bind _asbase_player_char_interface (Utilities|Casting|CastToBasePlayerCharInterface (Components|GetOwner)))
    (Default|AddJourneyEventInterfaceCall _asbase_player_char_interface "EarnAPerk")))

(fn GetPerksBreathingTimerModifier
  (bind _asi_perk_system_interface (Utilities|Casting|CastToI_PerkSystemInterface (Actor|GetComponentbyClass (Components|GetOwner) "/Script/ConanSandbox.PerkSystemComponent"))
    (:then
      (bind _hasperk (Default|HasPerk _asi_perk_system_interface "Vitality_10"))
      (if _hasperk
        (return (Variables|Default|GetBreathingTimerModifier))
        (else
          _)))
    (:CastFailed
      _))
  (return 1.0))

(fn GetPerksClimbingStaminaCostModifier
  (return (Variables|Default|GetClimbingStaminaModifier)))

(fn GetPerksConcussiveDamageModifier
  (bind _hasperk (CallFunction|HasPerk "Strength_10"))
  (if _hasperk
    (return (Variables|Default|GetConcussiveDamageModifier))
    (else
      (return 1.0))))

(fn GetPerksCrippleModifier
  (return (Variables|Default|GetCrippleModifier)))

(fn GetPerksDamageModifier
  (params (Target :type Actor%20Object%20Reference) (DamageCauser :type Actor%20Object%20Reference) (HitLocation :type EHitlocation%20Enum :default "None") (AttackingActor :type Actor%20Object%20Reference))
  (bind _output_get (LocalVariables|SetLocalTargetActor Target))
  (LocalVariables|SetLocalDamageCauser DamageCauser)
  (LocalVariables|SetLocalHitLocation HitLocation)
  (bind _output_get_2 (LocalVariables|SetLocalAttackingActor AttackingActor))
  ;[1 1 1] Stop hitting yourself
  (if (== _output_get_2 _output_get)
    (return 1.0)
    (else
      (Utilities|FlowControl|Sequence
        (:then_0
          ;[1 1 1] Strength_20 Perk
          (bind _asi_perk_system_interface (Utilities|Casting|CastToI_PerkSystemInterface (Actor|GetComponentbyClass (LocalVariables|GetLocalAttackingActor) "BP_PerkSystemComponent_C")))
          (bind _hasperk (Default|HasPerk _asi_perk_system_interface "Strength_20"))
          (if _hasperk
            (if (> (Utilities|Array|Length (Actor|GetComponentsbyTag (LocalVariables|GetLocalTargetActor) "/Game/Systems/Buffs/01_BP_AC_Buff_Master.01_BP_AC_Buff_Master_C" "Detrimental_Status_Effect")) 0)
              (LocalVariables|SetLocalModifierValue (+ (LocalVariables|GetLocalModifierValue) (Variables|Default|GetDamageModifierToAfflicted))))))
        (:then_1
          ;[1 1 1] Strength_30 Perk
          (bind _asi_perk_system_interface_2 (Utilities|Casting|CastToI_PerkSystemInterface (Actor|GetComponentbyClass (LocalVariables|GetLocalAttackingActor) "BP_PerkSystemComponent_C")))
          (bind _hasperk_2 (Default|HasPerk _asi_perk_system_interface_2 "Strength_30"))
          (if _hasperk_2
            (bind _asis_base_bpcombat_interface (Utilities|Casting|CastToIsBaseBPCombatInterface (Components|GetOwner)))
            (bind _action (Default|GetCharacterAction _asis_base_bpcombat_interface))
            (switch Utilities|FlowControl|Switch|SwitchonE_CharacterActionType _action
              (:NewEnumerator0
                _)
              (:NewEnumerator2
                _)
              (:NewEnumerator4
                _)
              (:NewEnumerator6
                _))
            (LocalVariables|SetLocalModifierValue (+ (LocalVariables|GetLocalModifierValue) (Variables|Default|GetDamageModifierLightAttacks)))))
        (:then_2
          ;[1 1 1] Strength_40 Perk
          (bind _asi_perk_system_interface_3 (Utilities|Casting|CastToI_PerkSystemInterface (Actor|GetComponentbyClass (LocalVariables|GetLocalAttackingActor) "BP_PerkSystemComponent_C")))
          (bind _hasperk_3 (Default|HasPerk _asi_perk_system_interface_3 "Strength_40"))
          (if _hasperk_3
            (bind _asis_base_bpcombat_interface_2 (Utilities|Casting|CastToIsBaseBPCombatInterface (Components|GetOwner)))
            (bind _action_2 (Default|GetCharacterAction _asis_base_bpcombat_interface_2))
            (switch Utilities|FlowControl|Switch|SwitchonE_CharacterActionType _action_2
              (:NewEnumerator1
                _)
              (:NewEnumerator3
                _)
              (:NewEnumerator5
                _)
              (:NewEnumerator7
                _))
            (LocalVariables|SetLocalModifierValue (+ (LocalVariables|GetLocalModifierValue) (Variables|Default|GetDamageModifierHeavyAttacks)))))
        (:then_3
          ;[1 1 1] Strength_50 Perk
          (bind _asi_perk_system_interface_4 (Utilities|Casting|CastToI_PerkSystemInterface (Actor|GetComponentbyClass (LocalVariables|GetLocalAttackingActor) "BP_PerkSystemComponent_C")))
          (bind _hasperk_4 (Default|HasPerk _asi_perk_system_interface_4 "Strength_50"))
          (if _hasperk_4
            (if (> (Utilities|Array|Length (Actor|GetComponentsbyTag (Components|GetOwner) "/Game/Systems/Buffs/01_BP_AC_Buff_Master.01_BP_AC_Buff_Master_C" "berserk")) 0)
              (LocalVariables|SetLocalModifierValue (+ (LocalVariables|GetLocalModifierValue) (Variables|Default|GetDamageModifierWhileBerserking))))))
        (:then_4
          ;[1 1 1] Encumberance_10 Perk
          (bind _asi_perk_system_interface_5 (Utilities|Casting|CastToI_PerkSystemInterface (Actor|GetComponentbyClass (LocalVariables|GetLocalAttackingActor) "BP_PerkSystemComponent_C")))
          (bind _hasperk_5 (Default|HasPerk _asi_perk_system_interface_5 "Encumberance_10"))
          (if _hasperk_5
            (Utilities|Casting|CastToConanCharacter (LocalVariables|GetLocalAttackingActor))
            (bind _tier (Default|GetEncumbranceTier (Actor|GetComponentbyClass (LocalVariables|GetLocalAttackingActor) "/Game/Systems/Combat/EncumbranceSystem/BP_EncumbranceSystem.BP_EncumbranceSystem_C")))
            (if (Utilities|Enum|Equal(Enum) _tier "Tier4")
              (LocalVariables|SetLocalModifierValue (+ (LocalVariables|GetLocalModifierValue) (Variables|Default|GetDamageModifierWhileEncumbered))))))
        (:then_5
          ;[1 1 1] Accuracy_50 Perk
          (bind _asi_perk_system_interface_6 (Utilities|Casting|CastToI_PerkSystemInterface (Actor|GetComponentbyClass (LocalVariables|GetLocalAttackingActor) "BP_PerkSystemComponent_C")))
          (bind _hasperk_6 (Default|HasPerk _asi_perk_system_interface_6 "Accuracy_50"))
          (if _hasperk_6
            (Utilities|Casting|CastToBPI_BaseProjectile (LocalVariables|GetLocalDamageCauser))
            (if (Utilities|Enum|Equal(Enum) (LocalVariables|GetLocalHitLocation) (Utilities|Enum|LiteralenumEHitlocation "Head"))
              (LocalVariables|SetLocalModifierValue (+ (LocalVariables|GetLocalModifierValue) (Variables|Default|GetHeadshotDamageModifier))))))
        (:then_6
          (return (LocalVariables|GetLocalModifierValue)))))))

(fn GetPerksDamageReductionModifier
  (return (Variables|Default|GetDamageReduction)))

(fn GetPerksEncumberanceModifier
  (return (Variables|Default|GetEncumberanceModifier)))

(fn GetPerksGotHitDurabilityModifier
  (return (Variables|Default|GetGotHitDurabilityModifier)))

(fn GetPerksJumpStaminaCostModifier
  (return (Variables|Default|GetJumpStaminaModifier)))

(fn GetPerksPenetrationModifier
  (return (Variables|Default|GetWeaponPenetrationModifier)))

(fn GetPerksSprintingStaminaModifier
  (Variables|Default|SetSprintStaminaModifier 1.0)
  (bind _asi_perk_system_interface (Utilities|Casting|CastToI_PerkSystemInterface (Actor|GetComponentbyClass (Components|GetOwner) "/Script/ConanSandbox.PerkSystemComponent")))
  (bind _hasperk (Default|HasPerk _asi_perk_system_interface "Agility_10"))
  (if _hasperk
    (bind _output_get (Variables|Default|SetSprintStaminaModifier (- (Variables|Default|GetSprintStaminaModifier) 0.1))))
  (return _output_get))

(fn GetPerksStaminaLightAttackModifier
  (params (ActionType :type E_CharacterActionType%20Enum :default "NewEnumerator0"))
  (bind _asi_perk_system_interface (Utilities|Casting|CastToI_PerkSystemInterface (Actor|GetComponentbyClass (Components|GetOwner) "BP_PerkSystemComponent_C"))
    (:then
      (bind _hasperk (Default|HasPerk _asi_perk_system_interface "Grit_40"))
      (if _hasperk
        (switch Utilities|FlowControl|Switch|SwitchonE_CharacterActionType ActionType
          (:NewEnumerator0
            (return (Variables|Default|GetStaminaLightAttackModifier)))
          (:NewEnumerator1
            _)
          (:NewEnumerator2
            (return (Variables|Default|GetStaminaLightAttackModifier)))
          (:NewEnumerator3
            _)
          (:NewEnumerator4
            (return (Variables|Default|GetStaminaLightAttackModifier)))
          (:NewEnumerator5
            _)
          (:NewEnumerator6
            (return (Variables|Default|GetStaminaLightAttackModifier)))
          (:NewEnumerator7
            _))))
    (:CastFailed
      _))
  (return 1.0))

(fn GetPerksStaminaModifierWhileNotEncumbered
  (return (Variables|Default|GetAttackStaminaModifierWhileNotEncumbered)))

(fn GetPerksStaminaRegenModifier
  (return (Variables|Default|GetStaminaRegenModifier)))

(fn GetRangedDamageModifier
  (bind _hasperk (CallFunction|HasPerk "Accuracy_30"))
  (if _hasperk
    (return 1.25)
    (else
      (return 1.0))))

(fn HasPerk
  (params (Perk :type Name))
  (bind _returnvalue (Class|PerkSystemComponent|HasOwnedPerk Perk))
  (return _returnvalue))